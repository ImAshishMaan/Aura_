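; BP_Slingshot_Rock is the rock for the enemy slingshot ability, and this graph only makes its mesh tumble.
; BeginPlay picks random yaw, pitch and roll rates in either direction.
; Tick adds local rotation to RockMesh using delta time for pitch and yaw, while the roll rate is multiplied by zero and has no effect.
; The graph holds no movement or hit logic.
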(event `self.ReceiveBeginPlay`
  (bind _returnvalue (`KismetMathLibrary.RandomFloatInRange` -360.0 360.0))
  (set `self.YawRotationRate` _returnvalue)
  (set `self.PichRR` _returnvalue)
  (set `self.RollRR` _returnvalue))

(event `self.ReceiveTick`
  (params (DeltaSeconds :type "Float (single-precision)"))
  (`SceneComponent.K2_AddLocalRotation` (`self.RockMesh`) (`KismetMathLibrary.MakeRotator` (* 0.0 (`self.RollRR`)) (* DeltaSeconds (`self.PichRR`)) (* DeltaSeconds (`self.YawRotationRate`))) false false))

(fn `UserConstructionScript`)