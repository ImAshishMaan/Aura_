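; GA_MeleeAttack is a gameplay ability for a spear melee attack on a combat target, apparently for AI characters.
; It faces the avatar toward the target, plays the attack montage and waits for its melee gameplay event.
; On that event it gathers live players in a small radius around the combat socket.
; CauseDamage follows the empty loop, hitting only the last element, then the ability ends after a short delay.
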(event `self.K2_ActivateAbility`
  (bind _returnvalue (`self.GetAvatarActorFromActorInfo`))
  (bind _returnvalue_2 (`self.GetAvatarActorFromActorInfo`))
  ;[1 1 1] It got set in Behaviour tree
  (bind _returnvalue_3 (message `EnemyInterface.GetCombatTarget` _returnvalue))
  (bind _ascombat_interface (cast `CombatInterface` _returnvalue))
  (`CombatInterface.UpdateFacingTarget` _ascombat_interface (`Actor.K2_GetActorLocation` _returnvalue_3))
  (`AbilityTask_PlayMontageAndWait.CreatePlayMontageAndWaitProxy` "None" "/Game/Assets/Enemies/Goblin/Animations/Spear/AM_Attack_Spear.AM_Attack_Spear"
    (:`then`
      (`AbilityTask_WaitGameplayEvent.WaitGameplayEvent` (struct :`TagName` "Event.Montage.Attack.Melee") null
        (:`EventReceived`
          (bind _returnvalue_4 (message `CombatInterface.GetCombatSocketLocation` _returnvalue_2))
          (bind _outoverlappingactors (`AuraAbilitySystemLibrary.GetLivePlayersWithinRadius` self (`|MakeArray` _returnvalue_2) 50.0 _returnvalue_4))
          (for _array_element _outoverlappingactors
            _)
          (`self.CauseDamage` _array_element)
          (`KismetSystemLibrary.Delay` 1.0)
          (`self.K2_EndAbility`))))))